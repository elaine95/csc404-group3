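; Player character Blueprint with movement and look input, a child-actor BowCaster it fires, and health reduced by overlapping Bolt actors.
; BeginPlay stores the spawn transform, creates the InGameHUD and resets health.
; Zero health or the K key destroys the actor.
; Its bound OnDestroyed handler delays, spawns and possesses a new Player at the stored transform, then calls Respawn to rerun the BeginPlay setup.
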(event Custom|TakeDamage
  (params (damage :type Integer))
  (bind _output_get (Variables|Default|SetHealth (- (Variables|Default|GetHealth) damage)))
  (if (<= _output_get 0)
    (Actor|DestroyActor)))

(event Custom|OnDestroyed_Event_0
  (params (DestroyedActor :type Actor%20Object%20Reference))
  (Utilities|FlowControl|Delay 0.5)
  (bind _returnvalue (Game|SpawnActorfromClass "Player_C" (Variables|Default|GetSpawn%20Transform) "Undefined" 0 0 0))
  (Pawn|Possess (Game|GetPlayerController 0) _returnvalue)
  (CallFunction|Respawn))

(event Custom|Respawn
  (Utilities|FlowControl|Sequence
    (:then_0
      (bind _asplayer (Utilities|Casting|CastToPlayer (Game|GetPlayerCharacter 0)))
      (Game|BindEventtoOnDestroyed _asplayer (delegate Custom|OnDestroyed_Event_0)))
    (:then_1
      (Utilities|Casting|CastToBowCasterGameMode (Game|GetGameMode))
      (Variables|Default|SetSpawn%20Transform (Transformation|GetActorTransform)))
    (:then_2
      ;[1 1 1] Create HUD
      (bind _returnvalue (UserInterface|CreateWidget "/Game/HUD/InGameHUD.InGameHUD_C"))
      (bind _output_get (Variables|Default|SetHealth%20Bar _returnvalue))
      (UserInterface|Viewport|AddtoPlayerScreen _output_get))
    (:then_3
      (Variables|Default|SetHealth 100))))

(event EventBeginPlay
  (Utilities|FlowControl|Sequence
    (:then_0
      (bind _asplayer (Utilities|Casting|CastToPlayer (Game|GetPlayerCharacter 0)))
      (Game|BindEventtoOnDestroyed _asplayer (delegate Custom|OnDestroyed_Event_0)))
    (:then_1
      (Utilities|Casting|CastToBowCasterGameMode (Game|GetGameMode))
      (Variables|Default|SetSpawn%20Transform (Transformation|GetActorTransform)))
    (:then_2
      ;[1 1 1] Create HUD
      (bind _returnvalue (UserInterface|CreateWidget "/Game/HUD/InGameHUD.InGameHUD_C"))
      (bind _output_get (Variables|Default|SetHealth%20Bar _returnvalue))
      (UserInterface|Viewport|AddtoPlayerScreen _output_get))
    (:then_3
      (Variables|Default|SetHealth 100))))

(event Collision|EventActorBeginOverlap
  (params (OtherActor :type Actor%20Object%20Reference))
  (if (== (Utilities|GetClass OtherActor) "/Game/Blueprints/Bolt.Bolt_C")
    (bind _asbolt (Utilities|Casting|CastToBolt OtherActor))
    (CallFunction|TakeDamage (Variables|/Game/Blueprints/Bolt.Bolt_C|GetDamage _asbolt))))

(event Input|ActionEvents|InputActionStartFire
  (params (Key :type Key%20Structure))
  (:Pressed
    (bind _asbow_caster (Utilities|Casting|CastToBowCaster (Variables|/Script/Engine.ChildActorComponent|GetChildActor (Variables|Default|GetBowCaster))))
    (Default|FireBow _asbow_caster)))

(event Input|AxisEvents|InputAxisTurn
  (params (AxisValue :type Float%20%28single-precision%29))
  ;[1 1 1] Look around
  (Pawn|Input|AddControllerYawInput AxisValue))

(event Input|AxisEvents|InputAxisLookup
  (params (AxisValue :type Float%20%28single-precision%29))
  ;[1 1 1] Look around
  (Pawn|Input|AddControllerPitchInput AxisValue))

(event Input|AxisEvents|InputAxisMoveToDirection
  (params (AxisValue :type Float%20%28single-precision%29))
  ;[1 1 1] Player movement
  (Pawn|Input|AddMovementInput (Math|Vector|GetForwardVector (Pawn|GetControlRotation :!class /Script/Engine.Pawn)) AxisValue false))

(event Input|KeyboardEvents|K
  (params (Key :type Key%20Structure))
  (:Pressed
    (Actor|DestroyActor)))

(fn ConstructionScript
  (Transformation|AttachActorToActor (Components|GetOwner (Variables|Default|GetBowCaster)) (Components|GetOwner (Variables|Default|GetStaticMesh)) "None" "KeepRelative" "KeepRelative" "KeepRelative" true))