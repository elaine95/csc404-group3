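; BowCaster is a weapon Blueprint that shoots Bolt actors when its FireBow event is called.
; Each call flashes a short-lived spark emitter at the actor's location, even during cooldown.
; A CanFire flag and delay rate-limit the shot and its laser sound.
; The Fire function spawns the bolt at the Arrow component's transform, shifted by an Offset rotated into the arrow's orientation.
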(event Custom|FireBow
  (Utilities|FlowControl|Sequence
    (:then_0
      (bind _returnvalue (Effects|SpawnEmitteratLocation "/Game/Art/Particles/FireSparks.FireSparks" (Transformation|GetActorLocation)))
      (Utilities|FlowControl|Delay 0.2)
      (Components|DestroyComponent _returnvalue))
    (:then_1
      (if (Variables|Default|GetCanFire)
        (Variables|Default|SetCanFire false)
        (CallFunction|Fire)
        (Audio|SpawnSoundatLocation "/Game/Art/Sound/321101__nsstudios__laser2.321101__nsstudios__laser2" (Transformation|GetActorLocation))
        (Utilities|FlowControl|Delay 0.8)
        (Variables|Default|SetCanFire true)))))

(event EventTick
  (params (DeltaSeconds :type Float%20%28single-precision%29)))

(fn ConstructionScript)

(fn Fire
  (bind _arrow (Variables|Default|GetArrow))
  (bind _returnvalue (Transformation|GetWorldRotation _arrow))
  (Game|SpawnActorfromClass "/Game/Blueprints/Bolt.Bolt_C" (Math|Transform|MakeTransform (+ (Transformation|GetWorldLocation _arrow) (Math|Vector|RotateVector (Variables|Default|GetOffset) _returnvalue)) _returnvalue) "Undefined" 0 0)
  (return))