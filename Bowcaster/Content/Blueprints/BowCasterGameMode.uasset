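; Game mode for BowCaster that runs a two-player local match with a countdown timer and a score.
; BeginPlay creates a second local player and adds an InGameHUD widget to each player's screen.
; Tick uses a one-second Delay to count down Minutes and Seconds, then pauses and opens the Endgame level at zero.
; KillScore adds kills to a single Score, not yet separated by player.
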(event Custom|KillScore
  (params (Kills :type Integer))
  ;[1 1 1] KillScore (TODO: Differentiate players)
  (Variables|Default|SetScore (+ Kills (Variables|Default|GetScore))))

(event EventBeginPlay
  ;[1 1 1] Initialize 2-player HUD
  (bind _returnvalue (UserInterface|CreateWidget "/Game/HUD/InGameHUD.InGameHUD_C"))
  (UserInterface|Viewport|AddtoPlayerScreen _returnvalue)
  (bind _returnvalue_2 (Class|GameplayStatics|CreatePlayer -1))
  (bind _returnvalue_3 (UserInterface|CreateWidget "/Game/HUD/InGameHUD.InGameHUD_C" _returnvalue_2))
  (UserInterface|Viewport|AddtoPlayerScreen _returnvalue_3))

(event EventTick
  (params (DeltaSeconds :type Float%20%28single-precision%29))
  ;[1 1 1] Timer
  (Utilities|FlowControl|Delay 1.0)
  (Variables|Default|Setseconds (- (Variables|Default|Getseconds) 1))
  (if (< (Variables|Default|Getseconds) 0)
    (Variables|Default|Setminutes (- (Variables|Default|Getminutes) 1))
    (Variables|Default|Setseconds 59))
  (if (== (Variables|Default|Getseconds) 0)
    (if (== (Variables|Default|Getminutes) 0)
      (Game|SetGamePaused true)
      (Game|OpenLevel(byName) "Endgame"))))

(fn ConstructionScript)